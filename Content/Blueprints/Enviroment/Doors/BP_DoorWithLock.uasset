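; Door Blueprint child that adds a lock, with a point light showing whether the door is locked.
; DoorOpen and DoorClose overrides only pass through to the parent door logic while IsLocked is false.
; SwitchLock toggles IsLocked and refreshes the light: brighter red when locked, dimmer green when unlocked.
; The construction script applies the same light update, so the initial lock state is visible on placement.
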(event `self.ReceiveActorBeginOverlap`
  (params (OtherActor :type "Actor Object Reference"))
  (`parent.ReceiveActorBeginOverlap` OtherActor))

(event `self.DoorOpen`
  (if (not (`self.IsLocked`))
    (`parent.DoorOpen`)))

(event `self.DoorClose`
  (if (not (`self.IsLocked`))
    (`parent.DoorClose`)))

(fn `SetLightProperties`
  (`LightComponent.SetIntensity` (`self.PointLight`) (select `bool` (`self.IsLocked`) :`false` 3000.0 :`true` 5000.0 :!type "Float (single-precision)"))
  (`LightComponent.SetLightColor` (`self.PointLight`) (select `bool` (`self.IsLocked`) :`false` (struct :`R` 0.098491 :`G` 0.495833 :`B` 0.017142 :`A` 1.0) :`true` (struct :`R` 0.604167 :`G` 0.000733 :`B` 0.024779 :`A` 1.0) :!type "LinearColor Structure") true))

(fn `SwitchLock`
  (set `self.IsLocked` (not (`self.IsLocked`)))
  (`self.SetLightProperties`))

(fn `UserConstructionScript`
  (`parent.UserConstructionScript`)
  (`self.SetLightProperties`))